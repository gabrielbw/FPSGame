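; Deathmatch game mode for local multiplayer FPS, running matches through setup, pre-game, in-game and post-game stages via SwitchGameStage.
; Setup recreates local players, then pre-game spawns characters and polls readiness on Tick to start a countdown.
; A timed match follows, with respawns at random SpawnPoints; the team filter is unwired.
; Post-game compares kills to announce a winner or tie, though its input-disabling controller loop is disconnected.
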(event Custom|Post%20Game
  ;[1 1 1] Post Game
  (Variables|Default|SetCanRestartGame true)
  (bind _asfpscontroller (Utilities|Casting|CastToFPSController (stale _array_element)))
  (Input|DisableInput (Pawn|GetControlledPawn _asfpscontroller) _asfpscontroller)
  (CallFunction|CalculateWinner&EndGameText)
  (bind _returnvalue (UserInterface|CreateWidget "/Game/UI/Deathmatch_PostGame_Widget.Deathmatch_PostGame_Widget_C"))
  (bind _output_get (Variables|Default|SetPostGameWidget _returnvalue))
  (UserInterface|Viewport|AddtoViewport _output_get 0))

(event Custom|Set%20up%20Game
  (bind _postgamewidget (Variables|Default|GetPostGameWidget))
  ;[1 1 1] Game Setup
  (Utilities|IsValid _postgamewidget
    (:Is%20Valid
      (Widget|RemovefromParent _postgamewidget))
    (:Is%20Not%20Valid
      _))
  (Variables|Default|SetEndGameText "")
  (Utilities|Array|Clear (Variables|Default|GetTiePlayersText))
  (Utilities|Array|Clear (Variables|Default|GetKillsArray))
  (Utilities|Array|Clear (Variables|Default|GetTopScoreHolders))
  (CallFunction|SetupControllers 2)
  (CallFunction|SwitchGameStage "NewEnumerator1"))

(event Custom|test
  (bind _returnvalue (Class|GameplayStatics|CreatePlayer -1))
  (bind (_return_value _location _rotation) (CallFunction|CustomChoosePlayerStart))
  (bind _returnvalue_2 (Game|SpawnActorfromClass "/Game/Blueprint/Player/FPSPlayerCharacter.FPSPlayerCharacter_C" (Math|Transform|MakeTransform _location _rotation "1,1,1") "AdjustIfPossibleButAlwaysSpawn" 0 0))
  (Default|AddHUD _returnvalue_2 _returnvalue)
  (Pawn|Possess _returnvalue _returnvalue_2))

(event Custom|Pre%20Game
  ;[1 1 1] Pre Game
  (Variables|Default|SetCanRestartGame false)
  (CallFunction|SpawnCharacters)
  (bind _returnvalue (UserInterface|CreateWidget "/Game/UI/Deathmatch_PreGame_Widget.Deathmatch_PreGame_Widget_C"))
  (bind _output_get (Variables|Default|SetPreGameWidget _returnvalue))
  (UserInterface|Viewport|AddtoViewport _output_get 0))

(event Custom|Timer%20Tick
  ;[1 1 1] Game Timer
  (Variables|Default|SetTimeSec (- (Variables|Default|GetTimeSec) 1))
  (if (< (Variables|Default|GetTimeSec) 0)
    (Variables|Default|SetTimeMin (- (Variables|Default|GetTimeMin) 1))
    (Variables|Default|SetTimeSec 59))
  (if (== (+ (Variables|Default|GetTimeMin) (Variables|Default|GetTimeSec)) 0)
    (CallFunction|SwitchGameStage "NewEnumerator3")))

(event Custom|In%20Game
  ;[1 1 1] In Game
  (for _array_element (Variables|Default|GetControllers)
    (bind _asfpsplayer_character (Utilities|Casting|CastToFPSPlayerCharacter (Pawn|GetControlledPawn _array_element)))
    (Variables|/Game/Blueprint/Player/FPSPlayerCharacter.FPSPlayerCharacter_C|SetCanRespawn _asfpsplayer_character true)
    (Default|Respawn _asfpsplayer_character)
    (bind _asfpscontroller (Utilities|Casting|CastToFPSController _array_element))
    (Variables|/Game/Blueprint/Player/FPSController.FPSController_C|SetKills _asfpscontroller 0))
  (Variables|Default|SetTimeMin 5)
  (Variables|Default|SetTimeSec 0)
  (Utilities|Time|SetTimerbyFunctionName 0 "Timer Tick" 1.0 true)
  (bind _returnvalue (UserInterface|CreateWidget "/Game/UI/Deathmatch_InGame_Widget.Deathmatch_InGame_Widget_C"))
  (UserInterface|Viewport|AddtoViewport _returnvalue 0))

(event Custom|CountdownTimer
  (bind _pregamewidget (Variables|Default|GetPreGameWidget))
  ;[1 1 1] Countdown Timer
  (bind _output_get (Variables|Default|SetCountdownTimerSec (- (Variables|Default|GetCountdownTimerSec) 1)))
  (if (== _output_get 0)
    (Widget|RemovefromParent _pregamewidget)
    (for _array_element (Variables|Default|GetReadiedPlayers)
      (Variables|/Game/Blueprint/Player/FPSController.FPSController_C|SetReady _array_element false))
    (Class|KismetSystemLibrary|PauseTimer 0 "CountdownTimer")
    (CallFunction|SwitchGameStage "NewEnumerator2")
    (else
      (UserInterface|Animation|PlayAnimation _pregamewidget (Variables|/Game/UI/Deathmatch_PreGame_Widget.Deathmatch_PreGame_Widget_C|GetCountdownTick _pregamewidget) 0.0 1 "Forward" 1.0 false)
      (Audio|PlaySound2D "/Game/Sound/Beep.Beep" 1.0 1.0 0.0 0 0))))

(event EventBeginPlay
  (CallFunction|RemoveOtherPlayers)
  (CallFunction|SwitchGameStage "NewEnumerator0"))

(event EventTick
  (params (DeltaSeconds :type Float%20%28single-precision%29))
  (Utilities|FlowControl|Sequence
    (:then_1
      ;[1 1 1] Check Readied Players
      (if (Utilities|Enum|Equal(Enum) (Variables|Default|GetCurrent%20Game%20Stage) "NewEnumerator1")
        (CallFunction|CheckReadiedPlayers)
        (Math|Integer|CompareInt (Utilities|Array|Length (Variables|Default|GetReadiedPlayers)) (Utilities|Array|Length (Variables|Default|GetControllers))
          (:==
            (if (not (Class|KismetSystemLibrary|IsTimerActive 0 "CountdownTimer"))
              (Variables|Default|SetCountdownTimerSec 4)
              (Utilities|Time|SetTimerbyFunctionName 0 "CountdownTimer" 1.0 true)))
          (:<
            (Class|KismetSystemLibrary|PauseTimer 0 "CountdownTimer")))))))

(event EventPostLogin
  (params (NewPlayer :type Player%20Controller%20Object%20Reference))
  ;[1 1 1] Adding and removing controllers
  (Utilities|Array|Add (Variables|Default|GetControllers) NewPlayer))

(event EventOnLogout
  (params (ExitingController :type Controller%20Object%20Reference))
  ;[1 1 1] Adding and removing controllers
  (Utilities|Array|RemoveItem (Variables|Default|GetControllers) ExitingController))

(event EventOnRestartPlayer
  (params (NewPlayer :type Controller%20Object%20Reference))
  ;[1 1 1] Respawn
  (bind _asfpsplayer_character (Utilities|Casting|CastToFPSPlayerCharacter (Pawn|GetControlledPawn NewPlayer)))
  (bind _output_get (Variables|/Game/Blueprint/Player/FPSPlayerCharacter.FPSPlayerCharacter_C|SetisAlive _asfpsplayer_character true))
  (bind _output_get_2 (Variables|/Game/Blueprint/Player/FPSPlayerCharacter.FPSPlayerCharacter_C|SetPlayerMovable? _asfpsplayer_character _output_get))
  (Variables|/Game/Blueprint/Player/FPSPlayerCharacter.FPSPlayerCharacter_C|SetCameraMovable? _asfpsplayer_character _output_get_2)
  (Variables|/Game/Blueprint/Player/FPSPlayerCharacter.FPSPlayerCharacter_C|SetCanRespawn _asfpsplayer_character false)
  (Variables|/Game/Blueprint/Player/FPSPlayerCharacter.FPSPlayerCharacter_C|SetCurrentHealth _asfpsplayer_character (Variables|/Game/Blueprint/Player/FPSPlayerCharacter.FPSPlayerCharacter_C|GetHealthMax _asfpsplayer_character))
  (Default|UpdateHealth% _asfpsplayer_character 0.0)
  (Utilities|IsValid (Variables|/Game/Blueprint/Player/FPSPlayerCharacter.FPSPlayerCharacter_C|GetDeathWidget _asfpsplayer_character)
    (:Is%20Valid
      (Widget|RemovefromParent (Variables|/Game/Blueprint/Player/FPSPlayerCharacter.FPSPlayerCharacter_C|GetDeathWidget _asfpsplayer_character)))
    (:Is%20Not%20Valid
      _))
  (bind (_return_value _location _rotation) (CallFunction|CustomChoosePlayerStart NewPlayer))
  (Transformation|SetActorLocation _asfpsplayer_character _location false false)
  (Transformation|SetActorRotation _asfpsplayer_character _rotation)
  (Audio|PlaySound2D "/Game/Sound/Equip.Equip" 1.0 1.0 0.0 0 0 false))

(fn ConstructionScript)

(fn SetupControllers
  (params (Number%20of%20Players :type Integer))
  (for _array_element (Variables|Default|GetControllers)
    (Class|GameplayStatics|RemovePlayer (.AsPlayer%20Controller (Utilities|Casting|CastToPlayerController _array_element)) true)
    (Class|GameplayStatics|RemovePlayer (Game|GetPlayerController 0) true)
    (for _index (range 0 (- Number%20of%20Players 1))
      (bind _returnvalue (Class|GameplayStatics|CreatePlayer _index))
      (bind _asfpscontroller (Utilities|Casting|CastToFPSController _returnvalue))
      (Variables|/Game/Blueprint/Player/FPSController.FPSController_C|SetTeam _asfpscontroller "NewEnumerator2"))))

(fn SpawnCharacters
  (for _array_element (Variables|Default|GetControllers)
    (bind _return_value (CallFunction|CustomChoosePlayerStart _array_element))
    (bind _returnvalue (Game|SpawnActorfromClass "/Game/Blueprint/Player/FPSPlayerCharacter.FPSPlayerCharacter_C" (Math|Transform|MakeTransform (Transformation|GetActorLocation _return_value) (Transformation|GetActorRotation _return_value) "1,1,1") "AdjustIfPossibleButAlwaysSpawn" 0 0))
    (Utilities|IsValid _returnvalue
      (:Is%20Valid
        (Variables|/Game/Blueprint/Player/FPSPlayerCharacter.FPSPlayerCharacter_C|SetID _returnvalue (Class|GameplayStatics|GetPlayerControllerID (.AsFPSController (Utilities|Casting|CastToFPSController _array_element))))
        (Pawn|Possess (.AsFPSController (Utilities|Casting|CastToFPSController _array_element)) _returnvalue)
        (Audio|PlaySound2D "/Game/Sound/Equip.Equip" 1.0 1.0 0.0 0 0)))))

(fn RemoveOtherPlayers
  (for _index (range 1 3)
    (Utilities|IsValid (Class|GameplayStatics|GetPlayerControllerfromID _index)
      (:Is%20Valid
        (Class|GameplayStatics|RemovePlayer (Class|GameplayStatics|GetPlayerControllerfromID _index) true)))))

(fn SwitchGameStage
  (params (Game%20stage :type E_GameStage%20Enum :default "NewEnumerator0"))
  (bind _output_get (Variables|Default|SetCurrent%20Game%20Stage Game%20stage))
  (switch Utilities|FlowControl|Switch|SwitchonE_GameStage _output_get
    (:NewEnumerator0
      (CallFunction|SetUpGame))
    (:NewEnumerator1
      (CallFunction|PreGame))
    (:NewEnumerator2
      (CallFunction|InGame))
    (:NewEnumerator3
      (CallFunction|PostGame))))

(fn ChoosePlayerStart
  (params (Player :type Controller%20Object%20Reference))
  (bind _return_value (CallFunction|CustomChoosePlayerStart Player))
  (return _return_value))

(fn CustomChoosePlayerStart
  (params (Player :type Controller%20Object%20Reference))
  (bind _outactors (Actor|GetAllActorsOfClass "/Game/Blueprint/Player/SpawnPoint.SpawnPoint_C"))
  (bind _output_get (LocalVariables|SetSelected%20SpawnPoint (.OutItem (Utilities|Array|Random _outactors))))
  (return (LocalVariables|GetSelected%20SpawnPoint) (Transformation|GetActorLocation (LocalVariables|GetSelected%20SpawnPoint)) (Transformation|GetActorRotation (LocalVariables|GetSelected%20SpawnPoint))))

(fn CalculateWinner&EndGameText
  (bind _topscoreholders (Variables|Default|GetTopScoreHolders))
  (bind _tieplayerstext (Variables|Default|GetTiePlayersText))
  (for _array_element (Variables|Default|GetControllers)
    (bind _asfpscontroller (Utilities|Casting|CastToFPSController _array_element))
    (Utilities|Array|Add (Variables|Default|GetKillsArray) (Variables|/Game/Blueprint/Player/FPSController.FPSController_C|GetKills _asfpscontroller)))
  (Variables|Default|SetHighestScoreValue (.MaxValue (Math|Integer|MaxOfIntArray (Variables|Default|GetKillsArray))))
  (for _array_element_2 (Variables|Default|GetControllers)
    (bind _asfpscontroller_2 (Utilities|Casting|CastToFPSController _array_element_2))
    (Math|Integer|CompareInt (Variables|/Game/Blueprint/Player/FPSController.FPSController_C|GetKills _asfpscontroller_2) (Variables|Default|GetHighestScoreValue)
      (:==
        (Utilities|Array|Add _topscoreholders _asfpscontroller_2))))
  (if (> (Utilities|Array|Length _topscoreholders) 1)
    ;[1 1 1] Players Tie
    (for _array_element_3 (Variables|Default|GetTopScoreHolders)
      (Utilities|Array|Add _tieplayerstext (Utilities|String|ToString(Text) (Utilities|Text|FormatText "Player {ID} " (+ (Class|GameplayStatics|GetPlayerControllerID _array_element_3) 1)))))
    (bind _output_get (Variables|Default|SetEndGameText (Utilities|Text|FormatText "Tie between {Players}" (Class|BlueprintPathsLibrary|Combine _tieplayerstext))))
    (Development|PrintString (Utilities|String|ToString(Text) _output_get))
    (else
      (Variables|Default|SetEndGameText (Utilities|Text|FormatText "Player {ID} Wins!" (+ (Class|GameplayStatics|GetPlayerControllerID (Utilities|Array|Get(acopy) _topscoreholders)) 1))))))

(fn CheckReadiedPlayers
  (for _array_element (Variables|Default|GetControllers)
    (if (Variables|/Game/Blueprint/Player/FPSController.FPSController_C|GetReady (.AsFPSController (Utilities|Casting|CastToFPSController _array_element)))
      (if (not (Utilities|Array|ContainsItem (Variables|Default|GetReadiedPlayers) (.AsFPSController (Utilities|Casting|CastToFPSController _array_element))))
        (Utilities|Array|Add (Variables|Default|GetReadiedPlayers) (.AsFPSController (Utilities|Casting|CastToFPSController _array_element))))
      (elif (Utilities|Array|ContainsItem (Variables|Default|GetReadiedPlayers) (.AsFPSController (Utilities|Casting|CastToFPSController _array_element)))
        (Utilities|Array|RemoveItem (Variables|Default|GetReadiedPlayers) (.AsFPSController (Utilities|Casting|CastToFPSController _array_element)))))))

(fn CanEndCheck
  (if true
    (CallFunction|SwitchGameStage "NewEnumerator3")
    (return true)
    (else
      (return false))))