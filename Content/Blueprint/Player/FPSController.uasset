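; FPSController is a player controller Blueprint that handles restart and ready-up input for the deathmatch game mode.
; RestartGame asks GM_Deathmatch to switch to its first game stage, provided the mode allows a restart.
; ToggleReady flips the Ready flag, but only during one specific game stage.
; Both inputs cast the game mode directly, which exists only on the server, and do nothing if the cast fails.
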(event EventBeginPlay)

(event EventTick
  (params (DeltaSeconds :type Float%20%28single-precision%29)))

(event Input|ActionEvents|InputActionRestartGame
  (params (Key :type Key%20Structure))
  (:Pressed
    (bind _asgm_deathmatch (Utilities|Casting|CastToGM_Deathmatch (Game|GetGameMode)))
    (if (Variables|/Game/Blueprint/GM_Deathmatch.GM_Deathmatch_C|GetCanRestartGame _asgm_deathmatch)
      (Default|SwitchGameStage _asgm_deathmatch "NewEnumerator0"))))

(event Input|ActionEvents|InputActionToggleReady
  (params (Key :type Key%20Structure))
  (:Pressed
    (bind _asgm_deathmatch (Utilities|Casting|CastToGM_Deathmatch (Game|GetGameMode)))
    (if (Utilities|Enum|Equal(Enum) (Variables|/Game/Blueprint/GM_Deathmatch.GM_Deathmatch_C|GetCurrent%20Game%20Stage _asgm_deathmatch) "NewEnumerator1")
      (Variables|Default|SetReady (not (Variables|Default|GetReady))))))

(fn ConstructionScript)