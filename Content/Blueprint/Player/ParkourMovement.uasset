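; Parkour movement logic for the first-person player character, adding wall running, wall jumping and mantling.
; A looping timer traces both sides while falling, launches the character along valid walls and eases gravity, with timed suppression after each run.
; Jump events kick off walls and run staged wall, ledge and headroom traces, passing the mantle target and crouch requirement to FPSPlayerCharacter.
; Tick rolls the control rotation to match the move.
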(event Custom|Init
  (params (Character :type Character%20Object%20Reference))
  (bind _output_get (Variables|Default|SetCharacter Character))
  (bind _output_get_2 (Variables|Default|SetCharacter%20Movement (Variables|/Script/Engine.Character|GetCharacterMovement _output_get)))
  (Variables|Default|SetDefault%20Gravity (Variables|/Script/Engine.CharacterMovementComponent|GetGravityScale _output_get_2))
  (Utilities|Time|SetTimerbyEvent (delegate Custom|WallRunUpdateEvent) 0.02 true))

(event Custom|Jump%20Event
  (CallFunction|WallRunJump)
  (bind (_canmantle _targetlocation) (CallFunction|Mantle))
  (if _canmantle
    (Default|Mantle (.AsFPSPlayer%20Character (Utilities|Casting|CastToFPSPlayerCharacter (Variables|Default|GetCharacter))) (Transformation|GetActorLocation (Variables|Default|GetCharacter)) _targetlocation (Variables|Default|GetMustCrouch))))

(event Custom|Land%20Event
  (CallFunction|WallRunEnd 0.0)
  (Variables|Default|SetWallRunSuppressed? false))

(event Custom|WallRunUpdateEvent
  (if (not (Variables|Default|GetWallRunSuppressed?))
    (CallFunction|WallRunUpdate)))

(event Custom|ResetWallRunSuppression
  (Utilities|Time|ClearTimerbyFunctionName 0 "ResetWallRunSuppression")
  (Variables|Default|SetWallRunSuppressed? false))

(event EventBeginPlay)

(event EventTick
  (params (DeltaSeconds :type Float%20%28single-precision%29))
  (CallFunction|CameraTick))

(fn WallRunUpdate
  (bind _onwall (CallFunction|WallRunMovement (Transformation|GetActorLocation (Variables|Default|GetCharacter)) (.Right (Utilities|WallRunEndVectors)) -1.0))
  (if _onwall
    (bind _output_get (Variables|Default|SetWallRunning true))
    (Variables|Default|SetWallRunningR _output_get)
    (Variables|Default|SetWallRunningL false)
    (Variables|/Script/Engine.CharacterMovementComponent|SetGravityScale (Variables|Default|GetCharacter%20Movement) (Math|Interpolation|FInterpTo (Variables|/Script/Engine.CharacterMovementComponent|GetGravityScale (Variables|Default|GetCharacter%20Movement)) (Variables|Default|GetWallRunTargetGravity) (Utilities|Time|GetWorldDeltaSeconds) 1e+01) :!label _label)
    (elif (Variables|Default|GetWallRunningR)
      (CallFunction|WallRunEnd 1.0)
      (else
        (bind _onwall_2 (CallFunction|WallRunMovement (Transformation|GetActorLocation (Variables|Default|GetCharacter)) (.Left (Utilities|WallRunEndVectors)) 1.0))
        (if _onwall_2
          (Variables|Default|SetWallRunning true)
          (Variables|Default|SetWallRunningR false)
          (Variables|Default|SetWallRunningL true)
          (goto _label)
          (else
            (CallFunction|WallRunEnd 1.0)))))))

(fn WallRunMovement
  (params (Start :type Vector) (End :type Vector) (WallRunDirection :type Float%20%28single-precision%29))
  (bind _character (Variables|Default|GetCharacter))
  (bind _outhit (Collision|LineTraceByChannel Start End "TraceTypeQuery1" false 0 "None"))
  (if (.bblockinghit _outhit)
    (if (and (AI|Components|NavMovement|IsFalling (Variables|Default|GetCharacter%20Movement)) (.ReturnValue (Utilities|ValidWallRunVector (.normal _outhit))))
      (Variables|Default|SetWallRunNormal (.OutVec (Utilities|ValidWallRunVector (.normal _outhit))))
      (Character|LaunchCharacter (Variables|Default|GetCharacter) (Utilities|PlayertoWallVector) false false)
      (if (> (.z (Variables|/Script/Engine.MovementComponent|GetVelocity (Variables|Default|GetCharacter%20Movement))) 0.0)
        (Character|LaunchCharacter _character (* (Math|Vector|CrossProduct (Variables|Default|GetWallRunNormal) "0, 0,1.000000") (* (Variables|Default|GetWallRunSpeed) WallRunDirection)) true false)
        (else
          (Character|LaunchCharacter _character (* (Math|Vector|CrossProduct (Variables|Default|GetWallRunNormal) "0, 0,1.000000") (* (Variables|Default|GetWallRunSpeed) WallRunDirection)) true (Variables|Default|GetWallRunNoGravity))
          (if (Variables|Default|GetWallRunNoGravity)
            (Variables|Default|SetWallRunNoGravity false))))
      (return true)
      (else
        _)))
  (return false))

(fn WallRunEnd
  (params (Reset%20Time :type Float%20%28single-precision%29))
  (Variables|Default|SetWallRunNoGravity true)
  (if (Variables|Default|GetWallRunning)
    (Variables|Default|SetWallRunning false)
    (Variables|Default|SetWallRunningR false)
    (Variables|Default|SetWallRunningL false)
    (Variables|/Script/Engine.CharacterMovementComponent|SetGravityScale (Variables|Default|GetCharacter%20Movement) (Variables|Default|GetDefault%20Gravity))
    (CallFunction|SuppressWallRun Reset%20Time)))

(fn SuppressWallRun
  (params (Delay :type Float%20%28single-precision%29))
  (Variables|Default|SetWallRunSuppressed? true)
  (Utilities|Time|SetTimerbyFunctionName 0 "ResetWallRunSuppression" Delay))

(fn CameraTick
  (if (Variables|Default|GetMantling)
    (CallFunction|CameraTilt 7.0 8.0)
    (elif (Variables|Default|GetWallRunningL)
      (CallFunction|CameraTilt 15.0 1e+01)
      (elif (Variables|Default|GetWallRunningR)
        (CallFunction|CameraTilt -15.0 1e+01)
        (else
          (CallFunction|CameraTilt 0.0 1e+01))))))

(fn CameraTilt
  (params (Target%20X%20%28Roll%29 :type Float%20%28single-precision%29) (Speed :type Float%20%28single-precision%29))
  (bind _character (Variables|Default|GetCharacter))
  (bind _returnvalue (Pawn|GetController _character))
  (bind _returnvalue_2 (Pawn|GetControlRotation _returnvalue :!class /Script/Engine.Controller))
  (bind (_roll _pitch _yaw) (Math|Rotator|BreakRotator _returnvalue_2))
  (Pawn|SetControlRotation (Pawn|GetController (Variables|Default|GetCharacter)) (Math|Interpolation|RInterpTo _returnvalue_2 (Math|Rotator|MakeRotator Target%20X%20%28Roll%29 _pitch _yaw) (Utilities|Time|GetWorldDeltaSeconds) Speed)))

(fn WallRunJump
  (bind _wallrunnormal (Variables|Default|GetWallRunNormal))
  (bind _wallrunjumpoffforce (Variables|Default|GetWallRunJumpOffForce))
  (if (Variables|Default|GetWallRunning)
    (CallFunction|WallRunEnd 0.2)
    (Character|LaunchCharacter (Variables|Default|GetCharacter) (Math|Vector|MakeVector (* _wallrunjumpoffforce (.x _wallrunnormal)) (* _wallrunjumpoffforce (.y _wallrunnormal)) (Variables|Default|GetWallRunJumpHeight)) false true)))

(fn Mantle
  (bind _character (Variables|Default|GetCharacter))
  (bind _returnvalue (Transformation|GetActorLocation _character))
  (bind (_x _y _z) (Math|Vector|BreakVector _returnvalue))
  (bind _returnvalue_2 (+ _z 45.0))
  (bind _returnvalue_3 (Math|Vector|MakeVector _x _y _returnvalue_2))
  (if (AI|Components|NavMovement|IsCrouching (Variables|Default|GetCharacter%20Movement))
    (return false "0, 0, 0")
    (else
      (Utilities|FlowControl|Sequence
        (:then_0
          ;[1 1 1] Check for blocking wall
          (bind _outhit (Collision|CapsuleTraceByChannel _returnvalue_3 (+ _returnvalue_3 (* (Transformation|GetActorForwardVector _character) 3e+01)) 3e+01 88.0 "TraceTypeQuery1" false 0 "None"))
          (if (Math|Boolean|ANDBoolean (not (Class|CharacterMovementComponent|IsWalkable (Variables|Default|GetCharacter%20Movement) _outhit)) (not (.bBlockingHit (Collision|BreakHitResult _outhit))) (not (.bInitialOverlap (Collision|BreakHitResult _outhit))))
            (return false "0, 0, 0")
            (else
              (LocalVariables|SetInitialPoint (.ImpactPoint (Collision|BreakHitResult _outhit)))
              (LocalVariables|SetInitialNormal (.ImpactNormal (Collision|BreakHitResult _outhit))))))
        (:then_1
          ;[1 1 1] Trace Downwards for surface target location
          (bind _outhit_2 (Collision|SphereTraceByChannel (+ (+ (Math|Vector|MakeVector (.x (LocalVariables|GetInitialPoint)) (.y (LocalVariables|GetInitialPoint)) (- (.z (Transformation|GetActorLocation (Variables|Default|GetCharacter))) 45.0)) (* (LocalVariables|GetInitialNormal) -3e+01)) "0, 0,120.000000") (+ (Math|Vector|MakeVector (.x (LocalVariables|GetInitialPoint)) (.y (LocalVariables|GetInitialPoint)) (- (.z (Transformation|GetActorLocation (Variables|Default|GetCharacter))) 45.0)) (* (LocalVariables|GetInitialNormal) -3e+01)) 3e+01 "TraceTypeQuery1" false 0 "None"))
          (if (and (Class|CharacterMovementComponent|IsWalkable (Variables|Default|GetCharacter%20Movement) _outhit_2) (.bBlockingHit (Collision|BreakHitResult _outhit_2)))
            (LocalVariables|SetTargetLoc (.Location (Collision|BreakHitResult _outhit_2)))
            (else
              (return false "0, 0, 0"))))
        (:then_2
          ;[1 1 1] Check Room and Mantle
          (bind _hasroom (CallFunction|CheckMantleRoom (LocalVariables|GetTargetLoc)))
          (if _hasroom
            (if (Variables|Default|GetMustCrouch)
              (return true (LocalVariables|GetTargetLoc))
              (else
                (return true (Math|Vector|MakeVector (.x (LocalVariables|GetTargetLoc)) (.y (LocalVariables|GetTargetLoc)) (+ (.z (LocalVariables|GetTargetLoc)) (+ (Variables|/Script/Engine.CapsuleComponent|GetCapsuleHalfHeight (Variables|/Script/Engine.Character|GetCapsuleComponent (Variables|Default|GetCharacter))) 0.5))))))))))))

(fn CheckMantleRoom
  (params (TargetLocation :type Vector))
  (bind _character (Variables|Default|GetCharacter))
  (bind _capsulecomponent (Variables|/Script/Engine.Character|GetCapsuleComponent _character))
  (bind _outhit (Collision|SphereTraceByChannel (Math|Vector|MakeVector (.x TargetLocation) (.y TargetLocation) (+ (.z TargetLocation) 15.0)) (Math|Vector|MakeVector (.x TargetLocation) (.y TargetLocation) (+ (.z TargetLocation) (Variables|/Script/Engine.CapsuleComponent|GetCapsuleHalfHeight _capsulecomponent))) (Variables|/Script/Engine.CapsuleComponent|GetCapsuleRadius _capsulecomponent) "TraceTypeQuery1" false 0 "None"))
  (if (Math|Boolean|NORBoolean (.bBlockingHit (Collision|BreakHitResult _outhit)) (.bInitialOverlap (Collision|BreakHitResult _outhit)))
    (Variables|Default|SetMustCrouch false)
    (elif (<= (.Distance (Collision|BreakHitResult _outhit)) (- (Variables|/Script/Engine.CharacterMovementComponent|GetCrouchedHalfHeight (Variables|/Script/Engine.Character|GetCharacterMovement (Variables|Default|GetCharacter))) 15.0))
      (return false)
      (else
        (Variables|Default|SetMustCrouch true))))
  (Variables|Default|SetMantling true)
  (return true))