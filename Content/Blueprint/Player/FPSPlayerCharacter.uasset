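; First-person shooter player character with movement, hitscan pistol combat, health, death and respawn, plus per-player HUD.
; Input drives sprint with FOV kick, interpolated crouch camera and parkour through ParkourMovement, with a timeline-driven mantle.
; Shots trace from the camera; damage updates health, shows numbers to the attacker and credits kills on death.
; Timer-sampled look input drives weapon sway and recoil; possession assigns a scene-capture render target by player ID.
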(event Custom|GetMouseXY
  ;[1 1 1] WeaponSwayTimer
  (Variables|Default|SetMouseX (Input|AxisValues|GetPlayerLookLR))
  (Variables|Default|SetMouseY (Input|AxisValues|GetPlayerLookUD))
  ;;[1 1 1] Set Weapon Sway
  (Variables|Default|SetSwayX (Math|Float|MapRangeClamped (Variables|Default|GetMouseX) -1.0 1.0 -8.0 8.0))
  (if (Variables|Default|GetShooting?)
    (Variables|Default|SetSwayY (Variables|Default|GetRecoilAmount))
    (Utilities|FlowControl|Delay 0.08)
    (Variables|Default|SetShooting? false)
    (else
      (Variables|Default|SetSwayY (Math|Float|MapRangeClamped (Variables|Default|GetMouseY) -1.0 1.0 -5.0 5.0)))))

(event Custom|AddHUD
  (params (Controller :type Controller%20Object%20Reference))
  ;[1 1 1] Add HUD Widget
  (bind _asfpscontroller (Utilities|Casting|CastToFPSController Controller))
  (bind _returnvalue (UserInterface|CreateWidget "/Game/UI/HUD_Widget.HUD_Widget_C" _asfpscontroller))
  (bind _output_get (Variables|Default|SetHUD _returnvalue))
  (Variables|/Game/UI/HUD_Widget.HUD_Widget_C|SetOwning%20Player _output_get self)
  (UserInterface|Viewport|AddtoPlayerScreen _output_get))

(event Custom|Set%20Initials
  (bind _camera (Variables|Default|GetCamera))
  (bind _relativelocation (Variables|/Script/Engine.SceneComponent|GetRelativeLocation _camera))
  ;[1 1 1] Set Initials
  (bind _output_get (Variables|Default|SetCameraInitialRelativeLocation (Math|Vector|MakeVector (.x _relativelocation) (.y _relativelocation) (.z _relativelocation))))
  (Variables|Default|SetCurrentInterpLocation _output_get)
  (Variables|Default|SetInitialSkeletalMeshRelativeLoc (Variables|/Script/Engine.SceneComponent|GetRelativeLocation (Variables|Default|GetSkeletalMesh)))
  (Variables|Default|SetInitialFOV (Variables|/Script/Engine.CameraComponent|GetFieldOfView _camera)))

(event Custom|StartWeaponSwayTimer
  ;[1 1 1] WeaponSwayTimer
  (Utilities|Time|SetTimerbyEvent (delegate Custom|GetMouseXY) 0.1 true))

(event Custom|Mantle
  (params (StartPosition :type Vector) (TargetLocation :type Vector) (MustCrouch? :type Boolean))
  ;[1 1 1] Mantle
  (if MustCrouch?
    (Character|Crouch))
  (Pawn|Components|CharacterMovement|SetMovementMode (Variables|Character|GetCharacterMovement) "MOVE_Walking" 0)
  (bind _duration (Timeline|MantleTimeline PlayFromStart)
    (:Update
      (Transformation|SetActorLocation (Math|Vector|Lerp(Vector) StartPosition (+ TargetLocation (Math|Vector|GetForwardVector (Transformation|GetActorRotation))) _duration) false false))
    (:Finished
      (Pawn|Components|CharacterMovement|SetMovementMode (Variables|Character|GetCharacterMovement) "MOVE_Walking" 0)
      (Variables|/Game/Blueprint/Player/ParkourMovement.ParkourMovement_C|SetMantling (Variables|Default|GetParkourMovement) false)
      (Utilities|FlowControl|Delay 0.4)
      (Character|UnCrouch))))

(event Game|Damage|EventAnyDamage
  (params (Damage :type Float%20%28single-precision%29) (DamageType :type Damage%20Type%20Object%20Reference) (InstigatedBy :type Controller%20Object%20Reference) (DamageCauser :type Actor%20Object%20Reference))
  ;[1 1 1] ApplyDamage
  (if (Variables|Default|GetisAlive)
    (Utilities|FlowControl|Delay 0.1)
    (Audio|PlaySound2D "/Game/Sound/Grunt_Cue.Grunt_Cue" 1.0 1.0 0.0 0 0)
    (Camera|PlayWorldCameraShake "/Game/Blueprint/Player/MantleShake.MantleShake_C" (Transformation|GetWorldLocation (Variables|Default|GetCamera)) 0.0 2e+01)
    (CallFunction|UpdateHealth% Damage)
    (CallFunction|CheckAlive DamageCauser)
    (bind _asfpsplayer_character (Utilities|Casting|CastToFPSPlayerCharacter DamageCauser))
    (CallFunction|SpawnDamageText _asfpsplayer_character (Transformation|GetActorLocation) Damage (.AsFPSController (Utilities|Casting|CastToFPSController InstigatedBy)))
    (bind _float (Timeline|TakeDamage PlayFromStart)
      (:Update
        (Variables|Default|SetDamageIndicatorAlpha _float)))))

(event EventPossessed
  (params (NewController :type Controller%20Object%20Reference))
  (bind _scenecapturecomponent2d (Variables|Default|GetSceneCaptureComponent2D))
  (Variables|Default|SetMyController (.AsPlayer%20Controller (Utilities|Casting|CastToPlayerController NewController)))
  (Utilities|FlowControl|Sequence
    (:then_0
      (CallFunction|AddHUD NewController))
    (:then_1
      (Class|SceneCaptureComponent|HideComponent _scenecapturecomponent2d (Variables|Default|GetSkeletalMesh)))
    (:then_2
      (switch int (Variables|Default|GetID)
        (:0
          (Variables|/Script/Engine.SceneCaptureComponent2D|SetTextureTarget _scenecapturecomponent2d "/Game/Textures/Misc/PlayerCameraRT1.PlayerCameraRT1"))
        (:1
          (Variables|/Script/Engine.SceneCaptureComponent2D|SetTextureTarget _scenecapturecomponent2d "/Game/Textures/Misc/PlayerCameraRT2.PlayerCameraRT2"))
        (:2
          (Variables|/Script/Engine.SceneCaptureComponent2D|SetTextureTarget _scenecapturecomponent2d "/Game/Textures/Misc/PlayerCameraRT3.PlayerCameraRT3"))
        (:3
          (Variables|/Script/Engine.SceneCaptureComponent2D|SetTextureTarget _scenecapturecomponent2d "/Game/Textures/Misc/PlayerCameraRT4.PlayerCameraRT4"))))))

(event EventOnLanded
  (params (Hit :type Hit%20Result%20Structure%20%28by%20ref%29))
  ;[1 1 1] Basic Movement & Camera
  ;;[1 1 1] Jump/Crouch
  (Default|LandEvent (Variables|Default|GetParkourMovement)))

(event EventBeginPlay
  (Utilities|FlowControl|Sequence
    (:then_0
      (CallFunction|SetInitials))
    (:then_1
      (CallFunction|StartWeaponSwayTimer))
    (:then_2
      (CallFunction|UpdateHealth% 0.0))
    (:then_3
      (Default|Init (Variables|Default|GetParkourMovement) self))))

(event EventOnStartCrouch
  (params (HalfHeightAdjust :type Float%20%28single-precision%29) (ScaledHalfHeightAdjust :type Float%20%28single-precision%29))
  ;[1 1 1] Basic Movement & Camera
  ;;[1 1 1] Jump/Crouch
  ;;;[1 1 1] CrouchCameraMovement
  (Variables|Default|SetCurrentInterpLocation (+ (Variables|Default|GetCameraInitialRelativeLocation) (Math|Vector|MakeVector 0.0 0.0 ScaledHalfHeightAdjust)))
  (Variables|Default|SetSkeletalMeshHeightOffset (* (Variables|/Script/Engine.CharacterMovementComponent|GetCrouchedHalfHeight (Variables|Character|GetCharacterMovement)) -1.0))
  (Variables|Default|SetCameraInitialRelativeLocation (Math|Vector|MakeVector (.x (Variables|Default|GetCameraInitialRelativeLocation)) (.y (Variables|Default|GetCameraInitialRelativeLocation)) (- (.z (Variables|Default|GetCameraInitialRelativeLocation)) (/ (Variables|/Script/Engine.CharacterMovementComponent|GetCrouchedHalfHeight (Variables|Character|GetCharacterMovement)) 2.0)))))

(event EventOnEndCrouch
  (params (HalfHeightAdjust :type Float%20%28single-precision%29) (ScaledHalfHeightAdjust :type Float%20%28single-precision%29))
  ;[1 1 1] Basic Movement & Camera
  ;;[1 1 1] Jump/Crouch
  ;;;[1 1 1] CrouchCameraMovement
  (Variables|Default|SetCurrentInterpLocation (- (Variables|Default|GetCameraInitialRelativeLocation) (Math|Vector|MakeVector 0.0 0.0 ScaledHalfHeightAdjust)))
  (Variables|Default|SetSkeletalMeshHeightOffset (* (Components|Capsule|GetScaledCapsuleHalfHeight (Variables|Collision|GetCapsuleComponent)) -1.0))
  (Variables|Default|SetCameraInitialRelativeLocation (Math|Vector|MakeVector (.x (Variables|Default|GetCameraInitialRelativeLocation)) (.y (Variables|Default|GetCameraInitialRelativeLocation)) (+ (.z (Variables|Default|GetCameraInitialRelativeLocation)) (/ (Variables|/Script/Engine.CharacterMovementComponent|GetCrouchedHalfHeight (Variables|Character|GetCharacterMovement)) 2.0)))))

(event EventTick
  (params (DeltaSeconds :type Float%20%28single-precision%29))
  (bind _initialskeletalmeshrelativeloc (Variables|Default|GetInitialSkeletalMeshRelativeLoc))
  (Utilities|FlowControl|Sequence
    (:then_0
      (CallFunction|CameraTick))
    (:then_1
      (if (Variables|Default|GetPlayerMovable?)
        (CallFunction|ApplyWeaponSway)))
    (:then_2
      ;[1 1 1] Mesh Height Crouch
      (Transformation|SetRelativeLocation (Variables|Default|GetSkeletalMesh) (Math|Vector|MakeVector (.x _initialskeletalmeshrelativeloc) (.y _initialskeletalmeshrelativeloc) (Variables|Default|GetSkeletalMeshHeightOffset)) false false))))

(event Input|ActionEvents|InputActionJump
  (params (Key :type Key%20Structure))
  ;[1 1 1] Basic Movement & Camera
  ;;[1 1 1] Jump/Crouch
  (:Pressed
    (if (Variables|Default|GetPlayerMovable?)
      (Character|Jump)
      (Default|JumpEvent (Variables|Default|GetParkourMovement))))
  (:Released
    (Character|StopJumping)))

(event Input|ActionEvents|InputActionCrouch
  (params (Key :type Key%20Structure))
  ;[1 1 1] Basic Movement & Camera
  ;;[1 1 1] Jump/Crouch
  (:Pressed
    (if (Variables|Default|GetPlayerMovable?)
      (Character|Crouch)))
  (:Released
    (Character|UnCrouch)))

(event Input|ActionEvents|InputActionShoot
  (params (Key :type Key%20Structure))
  ;[1 1 1] Shoot
  (:Pressed
    (if (Variables|Default|GetPlayerMovable?)
      (Variables|Default|SetShooting? true)
      (Audio|PlaySound2D "/Game/Sound/Cue_Pistol_S.Cue_Pistol_S" 0.5 1.0 0.0 0 0 false)
      (Animation|Montage|PlayMontage (Variables|Default|GetSkeletalMesh) "/Game/Animation/Anim_Shoot_Montage.Anim_Shoot_Montage" 1.0 0.2
        (:then
          (bind _hitplayer (CallFunction|Shoot(:Hitscan)))
          (Utilities|FlowControl|Delay 0.1)
          (if (not _hitplayer)
            (Audio|PlaySound2D "/Game/Sound/Cue_Ricochet.Cue_Ricochet" 1.0 1.0 0.0 0 0)))))))

(event Input|ActionEvents|InputActionCrouchToggle
  (params (Key :type Key%20Structure))
  ;[1 1 1] Basic Movement & Camera
  ;;[1 1 1] Jump/Crouch
  (:Pressed
    (if (Variables|Default|GetPlayerMovable?)
      (if (AI|Components|NavMovement|IsCrouching (Variables|Character|GetCharacterMovement))
        (Character|UnCrouch)
        (else
          (Character|Crouch))))))

(event Input|ActionEvents|InputActionSprint
  (params (Key :type Key%20Structure))
  (bind _playermovable_ (Variables|Default|GetPlayerMovable?))
  ;[1 1 1] Basic Movement & Camera
  ;;[1 1 1] Sprint
  (:Pressed
    (if _playermovable_
      (Variables|Default|SetSprinting? true)
      (CallFunction|StartSprint)
      (if (Variables|Default|GetSprinting?) :!label _label
        (bind _fov_offset (Timeline|FOVTimeline PlayFromStart)
          (:Update
            (Camera|SetFieldOfView (Variables|Default|GetCamera) (+ _fov_offset (Variables|Default|GetInitialFOV)))))
        (else
          (Timeline|FOVTimeline ReverseFromEnd)))))
  (:Released
    (if _playermovable_
      (Variables|Default|SetSprinting? false)
      (CallFunction|StopSprint)
      (goto _label))))

(event Input|ActionEvents|InputActionRespawn
  (params (Key :type Key%20Structure))
  ;[1 1 1] Respawn
  (:Pressed
    (CallFunction|Respawn)))

(event Input|AxisEvents|InputAxisPlayerLookLR
  (params (AxisValue :type Float%20%28single-precision%29))
  ;[1 1 1] Basic Movement & Camera
  ;;[1 1 1] Camera
  (if (Variables|Default|GetCameraMovable?)
    (Pawn|Input|AddControllerYawInput (* AxisValue (Variables|Default|GetLookSensitivity)))))

(event Input|AxisEvents|InputAxisPlayerMoveFB
  (params (AxisValue :type Float%20%28single-precision%29))
  ;[1 1 1] Basic Movement & Camera
  ;;[1 1 1] Movement
  (if (Variables|Default|GetPlayerMovable?)
    (Pawn|Input|AddMovementInput (Math|Vector|GetForwardVector (Variables|Collision|GetCapsuleComponent)) AxisValue false)
    (Game|Feedback|ClientStartCameraShake (Game|GetPlayerController 0) "/Game/Blueprint/Player/HeadBob.HeadBob_C" (/ (Math|Vector|VectorLength (Pawn|Components|CharacterMovement|GetLastUpdateVelocity (Variables|Character|GetCharacterMovement))) (Variables|Default|GetWalkSpeed)) "CameraLocal" "0, 0, 0")))

(event Input|AxisEvents|InputAxisPlayerMoveLR
  (params (AxisValue :type Float%20%28single-precision%29))
  ;[1 1 1] Basic Movement & Camera
  ;;[1 1 1] Movement
  (if (Variables|Default|GetPlayerMovable?)
    (Pawn|Input|AddMovementInput (Math|Vector|GetRightVector (Variables|Collision|GetCapsuleComponent)) AxisValue false)
    (Game|Feedback|ClientStartCameraShake (Game|GetPlayerController 0) "/Game/Blueprint/Player/HeadBob.HeadBob_C" (/ (Math|Vector|VectorLength (Pawn|Components|CharacterMovement|GetLastUpdateVelocity (Variables|Character|GetCharacterMovement))) (Variables|Default|GetWalkSpeed)) "CameraLocal" "0, 0, 0")))

(event Input|AxisEvents|InputAxisPlayerLookUD
  (params (AxisValue :type Float%20%28single-precision%29))
  ;[1 1 1] Basic Movement & Camera
  ;;[1 1 1] Camera
  (if (Variables|Default|GetCameraMovable?)
    (Pawn|Input|AddControllerPitchInput (* AxisValue (Variables|Default|GetLookSensitivity)))))

(event Input|KeyboardEvents|V
  (params (Key :type Key%20Structure))
  (bind _postprocess (Variables|Default|GetPostProcess))
  ;[1 1 1] Comment
  (:Pressed
    (Utilities|FlowControl|FlipFlop
      (:A
        (Variables|/Script/Engine.PostProcessComponent|SetBlendWeight _postprocess 0.0))
      (:B
        (Variables|/Script/Engine.PostProcessComponent|SetBlendWeight _postprocess 1.0)))))

(fn ConstructionScript
  (Transformation|AttachComponentToComponent (Variables|Default|GetWeaponMesh%28FromOutside%29) (Variables|Default|GetSkeletalMesh) "Hand_R_Socket" "KeepRelative" "KeepRelative" "KeepRelative" true))

(fn StartSprint
  (Variables|/Script/Engine.CharacterMovementComponent|SetMaxWalkSpeed (Variables|Character|GetCharacterMovement) (Variables|Default|GetSprintSpeed)))

(fn StopSprint
  (Variables|/Script/Engine.CharacterMovementComponent|SetMaxWalkSpeed (Variables|Character|GetCharacterMovement) (Variables|Default|GetWalkSpeed)))

(fn UpdateHealth%
  (params (Damage%20to%20take :type Float%20%28single-precision%29))
  (bind _output_get (Variables|Default|SetCurrentHealth (- (Variables|Default|GetCurrentHealth) Damage%20to%20take)))
  (Variables|Default|SetHealthPercentage (/ _output_get (Variables|Default|GetHealthMax))))

(fn CameraTick
  (bind _output_get (Variables|Default|SetCurrentInterpLocation (Math|Interpolation|VInterpTo (Variables|Default|GetCurrentInterpLocation) (Variables|Default|GetCameraInitialRelativeLocation) (Utilities|Time|GetWorldDeltaSeconds) 1e+01)))
  (Transformation|SetRelativeLocation (Variables|Default|GetCamera) _output_get false false))

(fn CameraLerp
  (params (Current :type Vector) (Target :type Vector) (Speed :type Float%20%28single-precision%29))
  (Transformation|SetRelativeLocation (Variables|Default|GetCamera) (Math|Interpolation|VInterpTo Current Target (Utilities|Time|GetWorldDeltaSeconds) Speed) false false))

(fn ApplyWeaponSway
  (bind _returnvalue (Utilities|Time|GetWorldDeltaSeconds))
  (bind _weaponmesh_inside_ (Variables|Default|GetWeaponMesh%28Inside%29))
  (bind _relativerotation (Variables|/Script/Engine.SceneComponent|GetRelativeRotation _weaponmesh_inside_))
  (Transformation|SetRelativeRotation _weaponmesh_inside_ (Math|Rotator|MakeRotator (.roll _relativerotation) (Math|Interpolation|FInterpTo (.pitch _relativerotation) (Variables|Default|GetSwayY) _returnvalue 0.0) (- (Math|Interpolation|FInterpTo (.yaw _relativerotation) (Variables|Default|GetSwayX) _returnvalue 0.0) 1.8e+02)) false false))

(fn CheckAlive
  (params (Damage%20Causer :type Actor%20Object%20Reference))
  (bind _output_get (Variables|Default|SetisAlive (> (Variables|Default|GetCurrentHealth) 0.0)))
  (if _output_get
    _
    (else
      (CallFunction|OnDeath Damage%20Causer)))
  (return))

(fn OnDeath
  (params (Damage%20Causer :type Actor%20Object%20Reference))
  (Variables|Default|SetPlayerMovable? false)
  (Variables|Default|SetCameraMovable? false)
  (bind _returnvalue (UserInterface|CreateWidget "/Game/UI/Death_Widget.Death_Widget_C" (Variables|Default|GetMyController)))
  (bind _output_get (Variables|Default|SetDeathWidget _returnvalue))
  (UserInterface|Viewport|AddtoPlayerScreen _output_get)
  (Variables|Default|SetCanRespawn true)
  (bind _asfpscontroller (Utilities|Casting|CastToFPSController (Pawn|GetController (.AsPawn (Utilities|Casting|CastToPawn Damage%20Causer)))))
  (Variables|/Game/Blueprint/Player/FPSController.FPSController_C|SetKills _asfpscontroller (+ (Variables|/Game/Blueprint/Player/FPSController.FPSController_C|GetKills _asfpscontroller) 1)))

(fn Respawn
  (if (Variables|Default|GetCanRespawn)
    (Class|GameModeBase|RestartPlayer (Game|GetGameMode) (Variables|Default|GetMyController))))

(fn Shoot(Projectile)
  (bind _camera (Variables|Default|GetCamera))
  (bind _weaponmesh_inside_ (Variables|Default|GetWeaponMesh%28Inside%29))
  (bind _returnvalue (Transformation|GetWorldLocation _camera))
  (bind _returnvalue_2 (Transformation|GetSocketTransform _weaponmesh_inside_ "Barrel_End" "RTS_World"))
  (bind (_outhit _returnvalue_3) (Collision|LineTraceByChannel _returnvalue (+ _returnvalue (* (Math|Vector|GetForwardVector _camera) 1e+05)) "TraceTypeQuery1" false 0 "Persistent"))
  (if _returnvalue_3
    (bind _returnvalue_4 (Game|SpawnActorfromClass "/Game/Blueprint/Weapons/Bullet.Bullet_C" (Math|Transform|MakeTransform (.location _returnvalue_2) (Math|Rotator|FindLookatRotation (.location _returnvalue_2) (.location _outhit))) "AlwaysSpawn" 0 self))
    (Collision|IgnoreActorwhenMoving (Variables|Collision|GetCapsuleComponent) _returnvalue_4 false)
    (else
      (bind _returnvalue_5 (Game|SpawnActorfromClass "/Game/Blueprint/Weapons/Bullet.Bullet_C" (Math|Transform|MakeTransform (.location _returnvalue_2) (Transformation|GetWorldRotation (Variables|Default|GetCamera))) "AlwaysSpawn" 0 self))
      (Collision|IgnoreActorwhenMoving (Variables|Collision|GetCapsuleComponent) _returnvalue_5 false))))

(fn Shoot(:Hitscan)
  (bind _shootdamagemargin (Variables|Default|GetShootDamageMargin))
  (bind _camera (Variables|Default|GetCamera))
  (bind _returnvalue (Transformation|GetWorldLocation _camera))
  (bind (_outhit _returnvalue_2) (Collision|LineTraceByChannel _returnvalue (+ _returnvalue (* (Math|Vector|GetForwardVector _camera) 1e+05)) "TraceTypeQuery1" false 0 "None"))
  (if _returnvalue_2
    (if (or (== (Utilities|GetClass (.hitactor _outhit)) "FPSPlayerCharacter_C") (== (Utilities|GetClass (.hitactor _outhit)) "/Game/Blueprint/Enemy/AICharacter_Police.AICharacter_Police_C"))
      (Game|Damage|ApplyDamage (.hitactor _outhit) (Math|Conversions|ToFloat(Integer) (Math|Float|Ceil (+ (Variables|Default|GetShootDamageBase) (Math|Random|RandomFloatinRange (* _shootdamagemargin -1.0) _shootdamagemargin)))) 0 self)
      (Niagara|SpawnSystematLocation "/Game/Particle/NS_Blood.NS_Blood" (.location _outhit) (Math|Conversions|RotationFromXVector (.normal _outhit)))
      (return true)
      (else
        (Niagara|SpawnSystematLocation "/Game/Particle/NS_Sparks.NS_Sparks" (.location _outhit) (Math|Conversions|RotationFromXVector (.normal _outhit)))
        (return false)))))

(fn SpawnDamageText
  (params (SpawnLocation :type Vector) (IncomingDamage :type Float%20%28single-precision%29) (Instigator :type FPS%20Controller%20Object%20Reference))
  (bind _returnvalue (Pawn|GetController))
  (bind _asfpscontroller (Utilities|Casting|CastToFPSController _returnvalue))
  (bind _screenposition (Class|GameplayStatics|ProjectWorldtoScreen _asfpscontroller SpawnLocation true))
  (bind _returnvalue_2 (UserInterface|CreateWidget "/Game/UI/DamageNumber_Widget.DamageNumber_Widget_C" _asfpscontroller (Math|Vector2D|MakeVector2D (+ (.x _screenposition) 2e+01) (+ (.y _screenposition) -2e+01)) IncomingDamage))
  (UserInterface|Viewport|AddtoPlayerScreen _returnvalue_2))

(fn GetPlayerStates
  (return (Variables|Default|GetisAlive) (Variables|Default|GetShooting?) (AI|Components|NavMovement|IsCrouching (Variables|Character|GetCharacterMovement))))