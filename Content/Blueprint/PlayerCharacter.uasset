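; First-person shooter player character with walking, sprinting, crouching, jumping, damage intake and a HUD health display.
; Shooting traces from the camera and spawns a Bullet at the gun's barrel socket, aimed at the hit point or along the view.
; Tick smooths crouch camera height, applies timer-sampled mouse sway with recoil to the gun, and adjusts sprint FOV.
; Movement drives speed-scaled head bob, and V toggles post-processing.
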(event Custom|GetMouseXY
  ;[1 1 1] WeaponSwayTimer
  (Variables|Default|SetMouseX (Input|AxisValues|GetPlayerLookLR))
  (Variables|Default|SetMouseY (Input|AxisValues|GetPlayerLookUD)))

(event Game|Damage|EventAnyDamage
  (params (Damage :type Float%20%28single-precision%29) (DamageType :type Damage%20Type%20Object%20Reference) (InstigatedBy :type Controller%20Object%20Reference) (DamageCauser :type Actor%20Object%20Reference))
  ;[1 1 1] ApplyDamage
  (Variables|Default|SetCurrentHealth (- (Variables|Default|GetCurrentHealth) Damage)))

(event EventBeginPlay
  (bind _camera (Variables|Default|GetCamera))
  (Utilities|FlowControl|Sequence
    (:then_0
      ;[1 1 1] Set Initials
      (bind _output_get (Variables|Default|SetCameraStartLocation (Variables|/Script/Engine.SceneComponent|GetRelativeLocation _camera)))
      (Variables|Default|SetCurrentInterpLocation _output_get)
      (Variables|Default|SetInitialFOV (Variables|/Script/Engine.CameraComponent|GetFieldOfView _camera)))
    (:then_1
      ;[1 1 1] WeaponSwayTimer
      (Utilities|Time|SetTimerbyEvent (delegate Custom|GetMouseXY) 0.1 true))
    (:then_2
      ;[1 1 1] HUD Widget
      (bind _returnvalue (UserInterface|CreateWidget "/Game/Blueprint/HUD_Widget.HUD_Widget_C" (Game|GetPlayerController 0)))
      (bind _output_get_2 (Variables|Default|SetHUD _returnvalue))
      (UserInterface|Viewport|AddtoViewport _output_get_2 0))))

(event EventOnStartCrouch
  (params (HalfHeightAdjust :type Float%20%28single-precision%29) (ScaledHalfHeightAdjust :type Float%20%28single-precision%29))
  ;[1 1 1] Basic Movement & Camera
  ;;[1 1 1] Jump/Crouch
  ;;;[1 1 1] CrouchCameraMovement
  (if (not (AI|Components|NavMovement|IsFalling (Variables|Character|GetCharacterMovement)))
    (Variables|Default|SetCurrentInterpLocation (+ (Variables|Default|GetCameraStartLocation) (Math|Vector|MakeVector 0.0 0.0 ScaledHalfHeightAdjust)))))

(event EventOnEndCrouch
  (params (HalfHeightAdjust :type Float%20%28single-precision%29) (ScaledHalfHeightAdjust :type Float%20%28single-precision%29))
  ;[1 1 1] Basic Movement & Camera
  ;;[1 1 1] Jump/Crouch
  ;;;[1 1 1] CrouchCameraMovement
  (if (not (AI|Components|NavMovement|IsFalling (Variables|Character|GetCharacterMovement)))
    (Variables|Default|SetCurrentInterpLocation (- (Variables|Default|GetCameraStartLocation) (Math|Vector|MakeVector 0.0 0.0 ScaledHalfHeightAdjust)))))

(event EventTick
  (params (DeltaSeconds :type Float%20%28single-precision%29))
  (bind _returnvalue (Utilities|Time|GetWorldDeltaSeconds))
  (bind _returnvalue_2 (Utilities|Time|GetWorldDeltaSeconds))
  (bind _gun (Variables|Default|GetGun))
  (bind _camera (Variables|Default|GetCamera))
  (bind _initialfov (Variables|Default|GetInitialFOV))
  (bind _returnvalue_3 (+ _initialfov 1e+01))
  (bind _relativerotation (Variables|/Script/Engine.SceneComponent|GetRelativeRotation _gun))
  (Utilities|FlowControl|Sequence
    (:then_0
      ;[1 1 1] Camera Interpolation Control
      (bind _output_get (Variables|Default|SetCurrentInterpLocation (Math|Interpolation|VInterpTo (Variables|Default|GetCurrentInterpLocation) (Variables|Default|GetCameraStartLocation) DeltaSeconds 1e+01)))
      (Transformation|SetRelativeLocation (Variables|Default|GetCamera) _output_get false false))
    (:then_1
      ;[1 1 1] Set Weapon Sway
      (Variables|Default|SetSwayX (Math|Float|MapRangeClamped (Variables|Default|GetMouseX) -1.0 1.0 -8.0 8.0))
      (if (Variables|Default|GetShooting?)
        (Variables|Default|SetSwayY (Variables|Default|GetRecoilAmount))
        (Utilities|FlowControl|Delay 0.08)
        (Variables|Default|SetShooting? false)
        (else
          (Variables|Default|SetSwayY (Math|Float|MapRangeClamped (Variables|Default|GetMouseY) -1.0 1.0 -5.0 5.0)))))
    (:then_2
      ;[1 1 1] Apply weapon sway
      (Transformation|SetRelativeRotation _gun (Math|Rotator|MakeRotator (.roll _relativerotation) (Math|Interpolation|FInterpTo (.pitch _relativerotation) (Variables|Default|GetSwayY) _returnvalue 0.0) (- (Math|Interpolation|FInterpTo (.yaw _relativerotation) (Variables|Default|GetSwayX) _returnvalue 0.0) 1.8e+02)) false false))
    (:then_3
      ;[1 1 1] Update Health
      (Variables|/Game/Blueprint/HUD_Widget.HUD_Widget_C|SetHealthPercentage (Variables|Default|GetHUD) (/ (Variables|Default|GetCurrentHealth) (Variables|Default|GetHealthMax))))
    (:then_4
      ;[1 1 1] FOV
      (if (Variables|Default|GetSprinting?)
        (Camera|SetFieldOfView _camera (Math|Interpolation|FInterpTo _initialfov _returnvalue_3 _returnvalue_2 0.1))
        (else
          (Camera|SetFieldOfView _camera (Math|Interpolation|FInterpTo _returnvalue_3 _initialfov _returnvalue_2 0.1)))))))

(event Input|ActionEvents|InputActionJump
  (params (Key :type Key%20Structure :default "None"))
  ;[1 1 1] Basic Movement & Camera
  ;;[1 1 1] Jump/Crouch
  (:Pressed
    (Character|Jump))
  (:Released
    (Character|StopJumping)))

(event Input|ActionEvents|InputActionCrouch
  (params (Key :type Key%20Structure :default "None"))
  ;[1 1 1] Basic Movement & Camera
  ;;[1 1 1] Jump/Crouch
  (:Pressed
    (Character|Crouch)
    (Variables|Default|SetCrouching? true))
  (:Released
    (Character|UnCrouch)
    (Variables|Default|SetCrouching? false)))

(event Input|ActionEvents|InputActionShoot
  (params (Key :type Key%20Structure :default "None"))
  (bind _camera (Variables|Default|GetCamera))
  (bind _gun (Variables|Default|GetGun))
  (bind _returnvalue (Transformation|GetWorldLocation _camera))
  (bind _returnvalue_2 (Transformation|GetSocketTransform _gun "Barrel_End" "RTS_World"))
  ;[1 1 1] Shoot
  (:Pressed
    (Variables|Default|SetShooting? true)
    (Audio|SpawnSoundatLocation "/Game/Sound/Cue_Pistol_S.Cue_Pistol_S" (Transformation|GetWorldLocation (Variables|Default|GetGun)) "0, 0, 0" 1.0 1.0 0.0 0 0)
    (bind (_outhit _returnvalue_3) (Collision|LineTraceByChannel _returnvalue (+ _returnvalue (* (Math|Vector|GetForwardVector _camera) 1e+05)) "TraceTypeQuery1" false 0 "None"))
    (if _returnvalue_3
      (bind _returnvalue_4 (Game|SpawnActorfromClass "/Game/Blueprint/Bullet.Bullet_C" (Math|Transform|MakeTransform (.location _returnvalue_2) (Math|Rotator|FindLookatRotation (.location _returnvalue_2) (.location _outhit))) "AlwaysSpawn" 0 self))
      (Collision|IgnoreActorwhenMoving (Variables|Collision|GetCapsuleComponent) _returnvalue_4 false)
      (else
        (bind _returnvalue_5 (Game|SpawnActorfromClass "/Game/Blueprint/Bullet.Bullet_C" (Math|Transform|MakeTransform (.location _returnvalue_2) (Transformation|GetWorldRotation (Variables|Default|GetCamera))) "AlwaysSpawn" 0 self))
        (Collision|IgnoreActorwhenMoving (Variables|Collision|GetCapsuleComponent) _returnvalue_5 false)))))

(event Input|ActionEvents|InputActionCrouchToggle
  (params (Key :type Key%20Structure :default "None"))
  ;[1 1 1] Basic Movement & Camera
  ;;[1 1 1] Jump/Crouch
  (:Pressed
    (if (Variables|Default|GetCrouching?)
      (Character|UnCrouch)
      (Variables|Default|SetCrouching? false)
      (else
        (Character|Crouch)
        (Variables|Default|SetCrouching? true)))))

(event Input|ActionEvents|InputActionSprint
  (params (Key :type Key%20Structure :default "None"))
  ;[1 1 1] Basic Movement & Camera
  ;;[1 1 1] Sprint
  (:Pressed
    (Variables|Default|SetSprinting? true)
    (CallFunction|StartSprint))
  (:Released
    (Variables|Default|SetSprinting? false)
    (CallFunction|StopSprint)))

(event Input|AxisEvents|InputAxisPlayerLookLR
  (params (AxisValue :type Float%20%28single-precision%29))
  ;[1 1 1] Basic Movement & Camera
  ;;[1 1 1] Camera
  (if (Variables|Default|GetCameraMovable?)
    (Pawn|Input|AddControllerYawInput (* AxisValue (Variables|Default|GetLookSensitivity)))))

(event Input|AxisEvents|InputAxisPlayerMoveFB
  (params (AxisValue :type Float%20%28single-precision%29))
  ;[1 1 1] Basic Movement & Camera
  ;;[1 1 1] Movement
  (if (Variables|Default|GetPlayerMovable?)
    (Pawn|Input|AddMovementInput (Math|Vector|GetForwardVector (Variables|Collision|GetCapsuleComponent)) (* AxisValue (Variables|Default|GetMoveSpeedMult)) false)
    (Game|Feedback|ClientStartCameraShake (Game|GetPlayerController 0) "/Game/Blueprint/HeadBob.HeadBob_C" (/ (Math|Vector|VectorLength (Pawn|Components|CharacterMovement|GetLastUpdateVelocity (Variables|Character|GetCharacterMovement))) (Variables|Default|GetWalkSpeed)) "CameraLocal" "0, 0, 0")))

(event Input|AxisEvents|InputAxisPlayerMoveLR
  (params (AxisValue :type Float%20%28single-precision%29))
  ;[1 1 1] Basic Movement & Camera
  ;;[1 1 1] Movement
  (if (Variables|Default|GetPlayerMovable?)
    (Pawn|Input|AddMovementInput (Math|Vector|GetRightVector (Variables|Collision|GetCapsuleComponent)) (* AxisValue (Variables|Default|GetMoveSpeedMult)) false)
    (Game|Feedback|ClientStartCameraShake (Game|GetPlayerController 0) "/Game/Blueprint/HeadBob.HeadBob_C" (/ (Math|Vector|VectorLength (Pawn|Components|CharacterMovement|GetLastUpdateVelocity (Variables|Character|GetCharacterMovement))) (Variables|Default|GetWalkSpeed)) "CameraLocal" "0, 0, 0")))

(event Input|AxisEvents|InputAxisPlayerLookUD
  (params (AxisValue :type Float%20%28single-precision%29))
  ;[1 1 1] Basic Movement & Camera
  ;;[1 1 1] Camera
  (if (Variables|Default|GetCameraMovable?)
    (Pawn|Input|AddControllerPitchInput (* AxisValue (Variables|Default|GetLookSensitivity)))))

(event Input|KeyboardEvents|V
  (params (Key :type Key%20Structure :default "None"))
  (bind _postprocess (Variables|Default|GetPostProcess))
  (:Pressed
    (Utilities|FlowControl|FlipFlop
      (:A
        (Variables|/Script/Engine.PostProcessComponent|SetBlendWeight _postprocess 0.0))
      (:B
        (Variables|/Script/Engine.PostProcessComponent|SetBlendWeight _postprocess 1.0)))))

(fn ConstructionScript)

(fn StartSprint
  (Variables|/Script/Engine.CharacterMovementComponent|SetMaxWalkSpeed (Variables|Character|GetCharacterMovement) (Variables|Default|GetSprintSpeed)))

(fn StopSprint
  (Variables|/Script/Engine.CharacterMovementComponent|SetMaxWalkSpeed (Variables|Character|GetCharacterMovement) (Variables|Default|GetWalkSpeed)))