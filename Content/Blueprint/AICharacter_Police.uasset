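; AI police character that fires bullets at the player from a hand-attached Glock.
; Its Shoot event, while alive, spawns a Bullet at the barrel socket aimed at the player.
; Any damage marks it dead, disables capsule collision and updates the IsAlive blackboard key, also set on BeginPlay.
; Tick optionally draws the shooting range as a debug sphere; the range check function and a line trace are unfinished.
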(event Custom|Shoot
  (bind _glock (Variables|Default|GetGlock))
  (bind _returnvalue (Transformation|GetSocketLocation _glock "Barrel_End"))
  ;[1 1 1] Shoot
  (if (Variables|Default|GetIsAlive)
    (Game|SpawnActorfromClass "/Game/Blueprint/Bullet.Bullet_C" (Math|Transform|MakeTransform _returnvalue (Math|Rotator|FindLookatRotation _returnvalue (Transformation|GetActorLocation (Game|GetPlayerCharacter 0)))) "AlwaysSpawn" 0 0)))

(event Game|Damage|EventAnyDamage
  (params (Damage :type Float%20%28single-precision%29) (DamageType :type Damage%20Type%20Object%20Reference) (InstigatedBy :type Controller%20Object%20Reference) (DamageCauser :type Actor%20Object%20Reference))
  (Variables|Default|SetIsAlive false)
  (Collision|SetCollisionEnabled (Variables|Collision|GetCapsuleComponent) "NoCollision")
  (AI|Components|Blackboard|SetValueasBool (AI|GetBlackboard 0) (Utilities|Name|MakeLiteralName "IsAlive") (Variables|Default|GetIsAlive)))

(event EventBeginPlay
  (AI|Components|Blackboard|SetValueasBool (AI|GetBlackboard 0) (Utilities|Name|MakeLiteralName "IsAlive") (Variables|Default|GetIsAlive)))

(event EventTick
  (params (DeltaSeconds :type Float%20%28single-precision%29))
  ;[1 1 1] Draw Range
  (if (Variables|Default|GetDrawRangeSphere)
    (Rendering|Debug|DrawDebugSphere (Transformation|GetActorLocation) (Variables|Default|GetShootingRange) 12 "(R=1.000000,G=1.000000,B=1.000000,A=1.000000)" 0.0 1.0)))

(fn ConstructionScript
  (Transformation|AttachComponentToComponent (Variables|Default|GetGlock) (Variables|Character|GetMesh) "Hand_R_Socket" "KeepRelative" "KeepRelative" "KeepRelative" true))

(fn CheckShootingRange
  (if (<= (Transformation|GetDistanceTo (Game|GetPlayerCharacter 0)) (Variables|Default|GetShootingRange))
    _))