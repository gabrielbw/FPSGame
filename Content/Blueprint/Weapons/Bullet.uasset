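; Bullet projectile actor that damages whatever its mesh overlaps, other than the instigator that fired it.
; On BeginPlay the static mesh ignores the instigator when moving.
; An overlap applies Damage with the instigator as causer, spawns Niagara sparks unless the hit actor is the FPS player or police AI character, then destroys the bullet.
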(event OnComponentBeginOverlap(StaticMesh)
  (params (OverlappedComponent :type Primitive%20Component%20Object%20Reference) (OtherActor :type Actor%20Object%20Reference) (OtherComp :type Primitive%20Component%20Object%20Reference) (OtherBodyIndex :type Integer) (bFromSweep :type Boolean) (SweepResult :type Hit%20Result%20Structure%20%28by%20ref%29))
  (bind _returnvalue (Utilities|GetClass OtherActor))
  (if (!= (Game|GetInstigator) OtherActor)
    (Game|Damage|ApplyDamage OtherActor (Variables|Default|GetDamage) 0 (Game|GetInstigator))
    (if (or (== _returnvalue "/Game/Blueprint/Player/FPSPlayerCharacter.FPSPlayerCharacter_C") (== _returnvalue "/Game/Blueprint/Enemy/AICharacter_Police.AICharacter_Police_C"))
      _
      (else
        (Niagara|SpawnSystematLocation "/Game/Particle/NS_Sparks.NS_Sparks" "0, 0, 0")))
    (Actor|DestroyActor)))

(event EventBeginPlay
  (Collision|IgnoreActorwhenMoving (Variables|Default|GetStaticMesh) (Game|GetInstigator) true))

(event Collision|EventActorBeginOverlap
  (params (OtherActor :type Actor%20Object%20Reference)))

(event EventTick
  (params (DeltaSeconds :type Float%20%28single-precision%29)))

(fn ConstructionScript)