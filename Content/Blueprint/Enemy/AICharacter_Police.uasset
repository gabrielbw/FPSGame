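; AI police enemy character that fires a Glock at player 0 and respawns after death.
; Shoot spawns a Bullet at the barrel socket aimed at the player.
; Damage reduces health and shows damage text; death disables collision, then a delayed respawn restores health at a GM_Deathmatch player start.
; IsAlive syncs to the Blackboard; OnDeath has kill-credit logic, but the damage event passes no DamageCauser to CheckAlive.
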(event Custom|Shoot
  (bind _glock (Variables|Default|GetGlock))
  (bind _returnvalue (Transformation|GetSocketLocation _glock "Barrel_End"))
  ;[1 1 1] Shoot
  (if (Variables|Default|GetIsAlive)
    (Audio|PlaySound2D "/Game/Sound/Cue_Pistol_Glock.Cue_Pistol_Glock" 0.5 1.0 0.0 0 0)
    (Game|SpawnActorfromClass "/Game/Blueprint/Weapons/Bullet.Bullet_C" (Math|Transform|MakeTransform _returnvalue (Math|Rotator|FindLookatRotation _returnvalue (Transformation|GetActorLocation (Game|GetPlayerCharacter 0)))) "AlwaysSpawn" 0 0)))

(event Game|Damage|EventAnyDamage
  (params (Damage :type Float%20%28single-precision%29) (DamageType :type Damage%20Type%20Object%20Reference) (InstigatedBy :type Controller%20Object%20Reference) (DamageCauser :type Actor%20Object%20Reference))
  (Utilities|FlowControl|Delay 0.1)
  (Audio|PlaySound2D "/Game/Sound/Grunt_Cue.Grunt_Cue" 1.0 1.0 0.0 0 0)
  (if (Variables|Default|GetisAlive)
    (CallFunction|UpdateHealth% Damage)
    (bind _asfpsplayer_character (Utilities|Casting|CastToFPSPlayerCharacter DamageCauser))
    (Default|SpawnDamageText _asfpsplayer_character (Transformation|GetActorLocation) Damage (.AsFPSController (Utilities|Casting|CastToFPSController InstigatedBy)))
    (bind _died (CallFunction|CheckAlive))
    (if _died
      (Utilities|FlowControl|Delay 2.0)
      (bind _asgm_deathmatch (Utilities|Casting|CastToGM_Deathmatch (Game|GetGameMode)))
      (bind _location (Default|CustomChoosePlayerStart _asgm_deathmatch))
      (Transformation|SetActorLocation _location false false)
      (Variables|Default|SetIsAlive true)
      (Collision|SetCollisionEnabled (Variables|Collision|GetCapsuleComponent) "QueryAndPhysics")
      (AI|Components|Blackboard|SetValueasBool (AI|GetBlackboard 0) (Utilities|Name|MakeLiteralName "IsAlive") (Variables|Default|GetIsAlive))
      (Variables|Default|SetCurrentHealth (Variables|Default|GetMaxHealth)))))

(event EventBeginPlay
  (AI|Components|Blackboard|SetValueasBool (AI|GetBlackboard 0) (Utilities|Name|MakeLiteralName "IsAlive") (Variables|Default|GetIsAlive))
  (Variables|Default|SetCurrentHealth (Variables|Default|GetMaxHealth)))

(event EventTick
  (params (DeltaSeconds :type Float%20%28single-precision%29))
  ;[1 1 1] Draw Range
  (if (Variables|Default|GetDrawRangeSphere)
    (Rendering|Debug|DrawDebugSphere (Transformation|GetActorLocation) (Variables|Default|GetShootingRange) 12 "(R=1.000000,G=1.000000,B=1.000000,A=1.000000)" 0.0 1.0)))

(fn ConstructionScript
  (Transformation|AttachComponentToComponent (Variables|Default|GetGlock) (Variables|Character|GetMesh) "Hand_R_Socket" "KeepRelative" "KeepRelative" "KeepRelative" true))

(fn CheckShootingRange
  (if (<= (Transformation|GetDistanceTo (Game|GetPlayerCharacter 0)) (Variables|Default|GetShootingRange))
    _))

(fn UpdateHealth%
  (params (Damage%20to%20take :type Float%20%28single-precision%29))
  (Variables|Default|SetCurrentHealth (- (Variables|Default|GetCurrentHealth) Damage%20to%20take)))

(fn CheckAlive
  (params (Damage%20Causer :type Actor%20Object%20Reference))
  (bind _output_get (Variables|Default|SetisAlive (> (Variables|Default|GetCurrentHealth) 0.0)))
  (if _output_get
    (return false)
    (else
      (CallFunction|OnDeath Damage%20Causer)
      (return true))))

(fn SpawnDamageText
  (params (SpawnLocation :type Vector) (IncomingDamage :type Float%20%28single-precision%29) (Instigator :type FPS%20Controller%20Object%20Reference)))

(fn OnDeath
  (params (Damage%20Causer :type Actor%20Object%20Reference))
  (Variables|Default|SetIsAlive false)
  (Collision|SetCollisionEnabled (Variables|Collision|GetCapsuleComponent) "NoCollision")
  (AI|Components|Blackboard|SetValueasBool (AI|GetBlackboard 0) (Utilities|Name|MakeLiteralName "IsAlive") (Variables|Default|GetIsAlive))
  (bind _asfpsplayer_character (Utilities|Casting|CastToFPSPlayerCharacter Damage%20Causer))
  (bind _asfpscontroller (Utilities|Casting|CastToFPSController (Pawn|GetController _asfpsplayer_character)))
  (Variables|/Game/Blueprint/Player/FPSController.FPSController_C|SetKills _asfpscontroller (+ (Variables|/Game/Blueprint/Player/FPSController.FPSController_C|GetKills _asfpscontroller) 1)))

(fn GetPlayerStates
  (return (Variables|Default|GetIsAlive) (Variables|Default|GetisShooting) (AI|Components|NavMovement|IsCrouching (Variables|Character|GetCharacterMovement))))