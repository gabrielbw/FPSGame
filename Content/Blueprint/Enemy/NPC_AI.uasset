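; AI controller for police NPCs that runs the NPC_BT behavior tree and decides when they shoot at the player.
; Perception updates set the CanSeePlayer blackboard key when the player is sensed and clear it after a five-second delay when lost.
; Each tick it writes InShootingRange from the distance to the player and turns the pawn's IsShooting on only when the player is both seen and in range.
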(event OnTargetPerceptionUpdated(AIPerception)
  (params (Actor :type Actor%20Object%20Reference) (Stimulus :type AI%20Stimulus%20Structure))
  (bind _returnvalue (AI|GetBlackboard 0))
  (bind _returnvalue_2 (Utilities|Name|MakeLiteralName "CanSeePlayer"))
  (Utilities|Casting|CastToFPSPlayerCharacter Actor)
  (if (.bSuccessfullySensed (Utilities|Struct|BreakAIStimulus Stimulus))
    (AI|Components|Blackboard|SetValueasBool _returnvalue _returnvalue_2 true)
    (else
      (Utilities|FlowControl|Delay 5.0)
      (AI|Components|Blackboard|SetValueasBool _returnvalue _returnvalue_2 false))))

(event EventBeginPlay
  (AI|RunBehaviorTree "/Game/Blueprint/Enemy/NPC_BT.NPC_BT"))

(event EventTick
  (params (DeltaSeconds :type Float%20%28single-precision%29))
  (bind _returnvalue (AI|GetBlackboard 0))
  (bind _returnvalue_2 (Pawn|GetControlledPawn))
  (bind _returnvalue_3 (Pawn|GetControlledPawn))
  (bind _asaicharacter_police (Utilities|Casting|CastToAICharacter_Police _returnvalue_2))
  (AI|Components|Blackboard|SetValueasBool _returnvalue (Utilities|Name|MakeLiteralName "InShootingRange") (<= (Math|Vector|Distance(Vector) (Transformation|GetActorLocation (Game|GetPlayerCharacter 0)) (Transformation|GetActorLocation _returnvalue_2)) (Variables|/Game/Blueprint/Enemy/AICharacter_Police.AICharacter_Police_C|GetShootingRange _asaicharacter_police)))
  (if (<= (Math|Vector|Distance(Vector) (Transformation|GetActorLocation (Game|GetPlayerCharacter 0)) (Transformation|GetActorLocation _returnvalue_2)) (Variables|/Game/Blueprint/Enemy/AICharacter_Police.AICharacter_Police_C|GetShootingRange _asaicharacter_police))
    (if (ScalableFloat|GetValueasBool _returnvalue (Utilities|Name|MakeLiteralName "CanSeePlayer"))
      (bind _asaicharacter_police_2 (Utilities|Casting|CastToAICharacter_Police _returnvalue_3))
      (Variables|/Game/Blueprint/Enemy/AICharacter_Police.AICharacter_Police_C|SetisShooting _asaicharacter_police_2 true)
      (else
        (bind _asaicharacter_police_3 (Utilities|Casting|CastToAICharacter_Police _returnvalue_3 :!label _label))
        (Variables|/Game/Blueprint/Enemy/AICharacter_Police.AICharacter_Police_C|SetisShooting _asaicharacter_police_3 false)))
    (else
      (goto _label))))

(fn ConstructionScript)